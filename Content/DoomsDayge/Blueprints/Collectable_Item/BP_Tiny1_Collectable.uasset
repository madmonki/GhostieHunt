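; BP_Tiny1_Collectable is a pickup item that counts toward winning the level.
; Its Interaction event decrements CollectablesLeft on the game mode, shows a pickup widget, plays a sound, then disables collision and hides the actor.
; At zero remaining, it waits briefly, stops the count widget, pauses, and shows the win menu with a cursor.
; Leftover overlap-input logic only disables input on end overlap; EnableInput is unwired.
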(event OnComponentEndOverlap(BoxCollision)
  (params (OverlappedComponent :type Primitive%20Component%20Object%20Reference) (OtherActor :type Actor%20Object%20Reference) (OtherComp :type Primitive%20Component%20Object%20Reference) (OtherBodyIndex :type Integer))
  ;[1 1 1] collecting with input. needs begin overlap and cast to bp as below
  (Utilities|Casting|CastToBP_FirstPersonCharacter OtherActor)
  (Input|DisableInput (Game|GetPlayerController 0)))

(event EventInteraction
  (bind _returnvalue (Game|GetPlayerController 0))
  (Utilities|Casting|CastToBP_FirstPersonCharacter (Game|Player|GetPlayerPawn 0))
  (bind _asbp_first_person_game_mode (Utilities|Casting|CastToBP_FirstPersonGameMode (Game|GetGameMode)))
  (bind _result (Math|Integer|DecrementInt (Variables|/Game/FirstPerson/Blueprints/BP_FirstPersonGameMode.BP_FirstPersonGameMode_C|GetCollectablesLeft _asbp_first_person_game_mode))
    (:%20%20
      (bind _output_get (Variables|/Game/FirstPerson/Blueprints/BP_FirstPersonGameMode.BP_FirstPersonGameMode_C|SetCollectablesLeft _asbp_first_person_game_mode _result))
      (bind _returnvalue_2 (UserInterface|CreateWidget "/Game/DoomsDayge/Blueprints/Collectable_Item/Widgets/CollectableWidgetBP.CollectableWidgetBP_C"))
      (UserInterface|Viewport|AddtoViewport _returnvalue_2 0)
      (Audio|PlaySound2D 0 1.0 1.0 0.0 0 0)
      (Collision|SetCollisionEnabled (Variables|Default|GetBoxCollision) "NoCollision")
      (Collision|SetCollisionEnabled (Variables|Default|GetStaticMesh) "NoCollision")
      (Rendering|SetActorHiddenInGame true)
      (if (== _output_get 0)
        (Utilities|FlowControl|Delay 0.6)
        (bind _asbp_first_person_game_mode_2 (Utilities|Casting|CastToBP_FirstPersonGameMode (Game|GetGameMode)))
        (Variables|/Game/DoomsDayge/Blueprints/Countdown.Countdown_C|SetIsCounting (Variables|/Game/FirstPerson/Blueprints/BP_FirstPersonGameMode.BP_FirstPersonGameMode_C|GetCountWid _asbp_first_person_game_mode_2) false)
        (Game|SetGamePaused true)
        (bind _returnvalue_3 (UserInterface|CreateWidget "/Game/DoomsDayge/Blueprints/GameOverMenu_UI/Widgets/WinMenu_Widget.WinMenu_Widget_C" _returnvalue))
        (UserInterface|Viewport|AddtoViewport _returnvalue_3 0)
        (Variables|/Script/Engine.PlayerController|SetbShowMouseCursor _returnvalue true)))))

(fn ConstructionScript)
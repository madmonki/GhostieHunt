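; BP_InspectParent is an inspectable actor, apparently a parent class, that the player picks up to view and then drops.
; Interacting with empty hands attaches it to the player's Item component, disables physics and collision, and places it InspectDistance ahead of the camera.
; It also enables its own input so IA_Drop can detach it, restore physics and collision, and clear CurrentItem.
; Input is never disabled afterwards.
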(event Input|EnhancedActionEvents|EnhancedInputActionIA_Drop
  (params (ActionValue :type Boolean) (ElapsedSeconds :type Float%20%28double-precision%29) (TriggeredSeconds :type Float%20%28double-precision%29) (InputAction :type Input%20Action%20Object%20Reference :default "/Game/DoomsDayge/Inputs/IA_Drop.IA_Drop"))
  (CallFunction|StopInspection)
  (Variables|/Game/FirstPerson/Blueprints/BP_FirstPersonCharacter.BP_FirstPersonCharacter_C|SetCurrentItem (stale EventInteractwith _output_get) 0))

(event EventBeginPlay)

(event Collision|EventActorBeginOverlap
  (params (OtherActor :type Actor%20Object%20Reference)))

(event EventTick
  (params (DeltaSeconds :type Float%20%28single-precision%29)))

(event EventInteractwith
  (params (PlayerCharacter :type BP%20First%20Person%20Character%20Object%20Reference))
  (bind _output_get (Variables|Default|SetPlayer%20Character PlayerCharacter))
  (Variables|/Game/FirstPerson/Blueprints/BP_FirstPersonCharacter.BP_FirstPersonCharacter_C|GetCurrentItem _output_get
    (:then)
    (:else
      (CallFunction|StartInspection))))

(fn ConstructionScript)

(fn StartInspection
  (bind _returnvalue (Game|GetPlayerCameraManager 0))
  (bind _inspectmesh (Variables|Default|GetInspectMesh))
  (Input|EnableInput (Game|GetPlayerController 0))
  (Transformation|AttachComponentToComponent (Variables|/Game/FirstPerson/Blueprints/BP_FirstPersonCharacter.BP_FirstPersonCharacter_C|GetItem (Variables|Default|GetPlayer%20Character)) "None" "SnapToTarget" "SnapToTarget" "KeepRelative" true)
  (Physics|SetSimulatePhysics _inspectmesh false)
  (Collision|SetCollisionEnabled _inspectmesh "NoCollision")
  (Variables|/Game/FirstPerson/Blueprints/BP_FirstPersonCharacter.BP_FirstPersonCharacter_C|SetCurrentItem (Variables|Default|GetPlayer%20Character) self)
  (Transformation|SetActorLocation (+ (Camera|GetCameraLocation _returnvalue) (* (Math|Vector|GetForwardVector (Camera|GetCameraRotation _returnvalue)) (Variables|Default|GetInspectDistance))) false false))

(fn StopInspection
  (bind _inspectmesh (Variables|Default|GetInspectMesh))
  (Transformation|DetachFromActor "KeepWorld" "KeepWorld" "KeepWorld")
  (Physics|SetSimulatePhysics _inspectmesh true)
  (Collision|SetCollisionEnabled _inspectmesh "QueryAndPhysics"))
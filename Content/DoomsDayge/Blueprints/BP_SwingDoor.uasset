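; BP_SwingDoor is a door that toggles in response to an Interaction event.
; The event gets the first-person player character and loops over swing doors overlapping its capsule.
; For each valid overlap it calls ToggleDoor on itself, not the overlapped door, passing the unit direction from player to this door.
; An equality check against self is left unused, and ToggleDoor's logic is defined outside these graphs.
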(event EventInteraction
  (bind _asbp_first_person_character (Utilities|Casting|CastToBP_FirstPersonCharacter (Game|Player|GetPlayerPawn 0)))
  (for _array_element (Collision|GetOverlappingActors (Variables|/Script/Engine.Character|GetCapsuleComponent _asbp_first_person_character) "BP_SwingDoor_C" :!class /Script/Engine.PrimitiveComponent)
    (if (Utilities|IsValid _array_element)
      (Class|SwingDoor|ToggleDoor self (Math|Vector|GetUnitDirection(Vector) (Transformation|GetActorLocation (Components|GetOwner (Variables|/Game/FirstPerson/Blueprints/BP_FirstPersonCharacter.BP_FirstPersonCharacter_C|GetFirstPersonCamera _asbp_first_person_character))) (Transformation|GetActorLocation self))))))

(fn ConstructionScript)
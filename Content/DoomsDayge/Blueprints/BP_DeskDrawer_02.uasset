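; BP_DeskDrawer_02 is an interactable desk drawer that slides open or closed on each Interaction event.
; It infers its state from the Drawer component's relative X, moving it a fixed distance back when at the open position, otherwise outward.
; Separate timelines for each direction lerp between cached start and end locations.
; The IsOpenable flag blocks further interaction until the slide finishes.
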(event EventInteraction
  (bind _drawer (Variables|Default|GetDrawer))
  (bind _drawer_2 (Variables|Default|GetDrawer))
  (bind _relativelocation (Variables|/Script/Engine.SceneComponent|GetRelativeLocation _drawer))
  (bind _relativelocation_2 (Variables|/Script/Engine.SceneComponent|GetRelativeLocation _drawer_2))
  (if (Variables|Default|GetIsOpenable)
    (Variables|Default|SetIsOpenable false)
    (if (Math|Float|NearlyEqual(Float) (.x (Variables|/Script/Engine.SceneComponent|GetRelativeLocation (Variables|Default|GetDrawer))) 3e+01 1e-06)
      (Variables|Default|SetStartLoc (Math|Vector|MakeVector (.x _relativelocation) (.y _relativelocation) (.z _relativelocation)))
      (Variables|Default|SetEndLoc (Math|Vector|MakeVector (+ (.x _relativelocation) -3e+01) (.y _relativelocation) (.z _relativelocation)))
      (bind _drawing (Timeline|Timeline_0 PlayFromStart)
        (:Update
          (Transformation|SetRelativeLocation (Variables|Default|GetDrawer) (Math|Vector|Lerp(Vector) (Variables|Default|GetStartLoc) (Variables|Default|GetEndLoc) _drawing) false false))
        (:Finished
          (Variables|Default|SetIsOpenable true)))
      (else
        (Variables|Default|SetStartLoc (Math|Vector|MakeVector (.x _relativelocation_2) (.y _relativelocation_2) (.z _relativelocation_2)))
        (Variables|Default|SetEndLoc (Math|Vector|MakeVector (+ (.x _relativelocation_2) 3e+01) (.y _relativelocation_2) (.z _relativelocation_2)))
        (bind _drawing_2 (Timeline|Timeline PlayFromStart)
          (:Update
            (Transformation|SetRelativeLocation (Variables|Default|GetDrawer) (Math|Vector|Lerp(Vector) (Variables|Default|GetStartLoc) (Variables|Default|GetEndLoc) _drawing_2) false false))
          (:Finished
            (Variables|Default|SetIsOpenable true)))))))

(fn ConstructionScript)